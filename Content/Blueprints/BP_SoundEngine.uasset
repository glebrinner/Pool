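; BP_SoundEngine is the sound manager for a billiards game, exposing events that play ball, cue, cushion, pocket and chalk sounds at given locations.
; Ball and cue hits pick soft, medium or hard sounds by splitting Power into thirds, and Power also sets the volume, as it does for cushion and pocket sounds.
; The chalk sound is kept as a component so a new chalk event or StopSounds can stop and destroy it.
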(event EventEmitCushionSound
  (params (location :type Vector :default "0, 0, 0") (power :type Float%20%28single-precision%29))
  (Audio|PlaySoundatLocation "/Game/Audio_16/S_Cushion.S_Cushion" location "0, 0, 0" power 1.0 0.0 0 0 0))

(event EventStopSounds
  (bind _chalksound (Variables|Default|GetchalkSound))
  (if (Utilities|IsValid _chalksound)
    (Audio|Components|Audio|Stop _chalksound)
    (Components|DestroyComponent _chalksound)))

(event EventEmitBalltoBallHitSound
  (params (location :type Vector :default "0, 0, 0") (power :type Float%20%28single-precision%29))
  (if (> power 0.6666)
    (Audio|PlaySoundatLocation "/Game/Audio_16/S_BallHard.S_BallHard" location "0, 0, 0" power 1.0 0.0 0 0 0)
    (elif (> power 0.3333)
      (Audio|PlaySoundatLocation "/Game/Audio_16/S_BallMedium.S_BallMedium" location "0, 0, 0" power 1.0 0.0 0 0 0)
      (else
        (Audio|PlaySoundatLocation "/Game/Audio_16/S_BallSoft.S_BallSoft" location "0, 0, 0" power 1.0 0.0 0 0 0)))))

(event EventEmitCueHitSound
  (params (location :type Vector :default "0, 0, 0") (power :type Float%20%28single-precision%29))
  (if (> power 0.6666)
    (Audio|PlaySoundatLocation "/Game/Audio_16/S_CueHard.S_CueHard" location "0, 0, 0" power 1.0 0.0 0 0 0)
    (elif (> power 0.3333)
      (Audio|PlaySoundatLocation "/Game/Audio_16/S_CueMedium.S_CueMedium" location "0, 0, 0" power 1.0 0.0 0 0 0)
      (else
        (Audio|PlaySoundatLocation "/Game/Audio_16/S_CueSoft.S_CueSoft" location "0, 0, 0" power 1.0 0.0 0 0 0)))))

(event EventEmitDropSound
  (params (location :type Vector :default "0, 0, 0") (power :type Float%20%28single-precision%29))
  (Audio|PlaySoundatLocation "/Game/Audio_16/S_Pocket.S_Pocket" location "0, 0, 0" power 1.0 0.0 0 0 0))

(event EventEmitChalkSound
  (params (location :type Vector :default "0, 0, 0"))
  (if (Utilities|IsValid (Variables|Default|GetchalkSound))
    (Audio|Components|Audio|Stop (Variables|Default|GetchalkSound))
    (Components|DestroyComponent (Variables|Default|GetchalkSound)))
  (bind _returnvalue (Audio|SpawnSoundatLocation "/Game/Audio_16/S_Chalk.S_Chalk" location "0, 0, 0" 1.0 1.0 0.0 0 0))
  (Variables|Default|SetchalkSound _returnvalue))

(fn ConstructionScript)
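; Game instance for a pool game client, acting as the hub for UI, level travel and in-app purchases.
; Registers all menus by name and Z-order with WidgetManager, caching them behind the loading screen while deferring the last ShowWidget request.
; Optional difficulty and stake prompts precede level opening, with user credentials and choices passed in the options string.
; Both IAP API versions feed Data.Shop for product info and receipt validation.
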(event Custom|Transition
  (CallFunction|HideWidget "ChooseDifficulty")
  (CallFunction|HideWidget "MainMenu")
  (bind _options (CallFunction|GetOptions))
  (Class|SefaPoolGameInstance|OpenLevel(byName) (Variables|Default|GetupcomingOpenLevel) _options))

(event Custom|RegisterDifficulty
  (params (diffLevel :type EDifficultyLevels%20Enum :default "DIFFICULTY_LEVEL_NONE"))
  (Variables|Default|SetDiffLevel diffLevel)
  (if (Variables|Default|GetShowStake)
    (CallFunction|ShowWidget "ChooseStake")
    (else
      (CallFunction|Transition))))

(event Custom|RegisterStake
  (params (Stake :type String))
  (Variables|Default|Setstake Stake)
  (CallFunction|Transition))

(event EventPullIAPInfoV1
  (params (iap_ids :type Array%20of%20Strings))
  (bind _inapppurchaseinformation (|InAppPurchaseQuery (Game|GetPlayerController 0) iap_ids)
    (:OnSuccess
      (Class|SefaPoolShop|ProcessIAPInfoV1 (Variables|/Script/SefaPool.SefaPoolData|Getshop (Variables|Default|Getdata)) _inapppurchaseinformation))))

(event EventOpenLevel
  (params (Level :type String) (Options :type String))
  (Development|PrintString (Utilities|String|Append "Opening level " Level "with options " Options) true true "(R=0.000000,G=0.660000,B=1.000000,A=1.000000)" 2e+02)
  (Class|SefaPoolGameInstance|ShowLoadingScreen)
  (Class|WidgetManager|HideonOpenLevel (Variables|Default|GetwidgetManager))
  (Utilities|FlowControl|Delay 0.2)
  (Game|OpenLevel(byName) (Utilities|String|StringToName Level) true Options))

(event EventPullIAPInfoV2
  (params (iap_ids :type Array%20of%20Strings))
  (bind _inappofferinformation (|InAppPurchaseQuery2 (Game|GetPlayerController 0) iap_ids)
    (:OnSuccess
      (Class|SefaPoolShop|ProcessIAPInfoV2 (Variables|/Script/SefaPool.SefaPoolData|Getshop (Variables|Default|Getdata)) _inappofferinformation))))

(event EventMakeinAppPurchaseV1
  (params (iap_id :type String) (consumable :type Boolean) (succesful :type Delegate%20%28by%20ref%29) (unsuccesful :type Delegate%20%28by%20ref%29))
  (bind _inapppurchasereceipts (|InAppPurchase (Game|GetPlayerController 0) (Utilities|Struct|MakeInAppPurchaseProductRequest iap_id consumable))
    (:OnSuccess
      (Class|SefaPoolShop|ValidateReceipt (Variables|/Script/SefaPool.SefaPoolData|Getshop (Variables|Default|Getdata)) (.identifier _inapppurchasereceipts) (.receiptdata _inapppurchasereceipts)))))

(event EventMakeinAppPurchaseV2
  (params (iap_id :type String) (consumable :type Boolean) (succesful :type Delegate%20%28by%20ref%29) (unsuccesful :type Delegate%20%28by%20ref%29))
  (bind _inapppurchasereceipts (|InAppPurchase2 (Game|GetPlayerController 0) (Utilities|Struct|MakeInAppPurchaseProductRequest2 iap_id consumable))
    (:OnSuccess
      (Class|SefaPoolShop|ValidateReceipt (Variables|/Script/SefaPool.SefaPoolData|Getshop (Variables|Default|Getdata)) (.itemid (Utilities|Array|Get(acopy) _inapppurchasereceipts)) (.validationinfo (Utilities|Array|Get(acopy) _inapppurchasereceipts))))))

(event EventShowPopup
  (params (title :type String) (description :type String) (button :type String))
  (bind _widget (CallFunction|GetWidget "Popup"))
  (bind _aspopup_widget_bp (Utilities|Casting|CastToPopupWidgetBP _widget))
  (Default|Fill _aspopup_widget_bp title description button)
  (CallFunction|ShowWidget "Popup"))

(event EventShowNewMessagePopup
  (params (message :type Remote%20Message%20Info%20Structure%20%28by%20ref%29))
  (bind _widget (CallFunction|GetWidget "NewRemoteMessage"))
  (bind _asfinal_new_remote_message_popup (Utilities|Casting|CastToFinalNewRemoteMessagePopup _widget))
  (Default|Populate _asfinal_new_remote_message_popup message)
  (CallFunction|ShowWidget "NewRemoteMessage"))

(event EventShowInteractivePopup
  (params (title :type String) (description :type String) (leftButton :type String) (rightButton :type String) (left :type Delegate%20%28by%20ref%29) (right :type Delegate%20%28by%20ref%29))
  (bind _widget (CallFunction|GetWidget "InteractivePopup"))
  (bind _asinteractive_popup_widget_bp (Utilities|Casting|CastToInteractivePopupWidgetBP _widget))
  (Default|Fill _asinteractive_popup_widget_bp title description leftButton rightButton)
  (Class|InteractivePopupWidget|RegisterCallbacks _asinteractive_popup_widget_bp left right)
  (CallFunction|ShowWidget "InteractivePopup"))

(event Custom|ConstructWidgets
  ;[1 1 1] Constructs every widget that exist in the game and initialize them to variables.
  (|Widgetconstrucrtionandinitializationtovariables))

(event Custom|ShowWidget
  (params (name :type String))
  (bind _returnvalue (Game|GetPlayerController 0))
  (if (Variables|Default|GetCaching)
    (Variables|Default|SetPostCachingShowWidget true)
    (Variables|Default|SetPostCachingWidgetName name)
    (Variables|Default|SetPostCachingLoadingScreenRemovalRequest true)
    (Utilities|IsValid _returnvalue
      (:Is%20Valid
        (Variables|/Script/Engine.PlayerController|SetbShowMouseCursor _returnvalue true)
        (Input|SetInputModeUIOnly _returnvalue 0 "LockInFullscreen")))
    (else
      (Class|WidgetManager|ShowWidget (Variables|Default|GetwidgetManager) name))))

(event Custom|HideWidget
  (params (Name :type String))
  (Class|WidgetManager|HideWidget (Variables|Default|GetwidgetManager) Name))

(event Custom|SwapWidgets
  (params (show_ :type String) (Hide_ :type String))
  (bind _widgetmanager (Variables|Default|GetwidgetManager))
  (Class|WidgetManager|ShowWidget _widgetmanager show_)
  (Class|WidgetManager|HideWidget _widgetmanager Hide_))

(event EventShowLoadingScreen
  (CallFunction|ShowWidget "Loading"))

(event EventHideLoadingScreen
  (if (Variables|Default|GetCaching)
    (Variables|Default|SetPostCachingLoadingScreenRemovalRequest true)
    (else
      (CallFunction|HideWidget "Loading"))))

(fn RemoveConnectingFailedfromParent
  (Widget|RemovefromParent (Variables|Textures|GetFailedToConnectWB)))

(fn RegisterUpcomingOpenLevel
  (params (addr :type String) (Stake :type Boolean) (Difficulty :type Boolean) (Options :type String))
  (Variables|Default|SetOptions Options)
  (Variables|Default|SetupcomingOpenLevel addr)
  (bind _output_get (Variables|Default|SetShowStake Stake))
  (if (or _output_get Difficulty)
    (if Difficulty
      (CallFunction|ShowWidget "ChooseDifficulty")
      (else
        (CallFunction|ShowWidget "ChooseStake")))
    (else
      (CallFunction|Transition))))

(fn GetDiff
  (return (Variables|Default|GetDiffLevel)))

(fn GetOptions
  (bind _aspool_client_game_instance (Utilities|Casting|CastToPoolClientGameInstance (Game|GetGameInstance)))
  (return (Utilities|String|Append (Utilities|String|Append (Variables|LobbyOptions|GetPlayerIdOptions) (.user_id (Utilities|Struct|BreakBackendInfo (Variables|/Script/SefaPool.PoolClientGameInstance|Getbackend_data _aspool_client_game_instance)))) (Utilities|String|Append (Variables|LobbyOptions|GetAccessTokenOptions) (.access_token (Utilities|Struct|BreakBackendInfo (Variables|/Script/SefaPool.PoolClientGameInstance|Getbackend_data _aspool_client_game_instance)))) (Utilities|String|Append (Variables|LobbyOptions|GetStakeOptions) (Variables|Default|Getstake)) (Utilities|String|Append (Variables|LobbyOptions|GetDifficultyOptions) (Utilities|String|ToString(Integer) (Math|Conversions|ToInteger(Byte) (Variables|Default|GetDiffLevel)))))))

(fn GetGameServerOptions
  (return ""))

(fn AddWidgettoView
  (params (Widget :type User%20Widget%20Object%20Reference))
  (bind _returnvalue (Game|GetPlayerController 0))
  (bind _output_get (LocalVariables|Setlocal_widget Widget))
  (if (Utilities|IsValid _output_get)
    _
    (else
      (bind _returnvalue_2 (UserInterface|CreateWidget (Utilities|GetClass _output_get) _returnvalue))
      (|SetBy-RefVar (LocalVariables|Getlocal_widget) _returnvalue_2)))
  (UserInterface|Viewport|AddtoViewport (LocalVariables|Getlocal_widget) 0)
  (Input|SetInputModeUIOnly _returnvalue (LocalVariables|Getlocal_widget) "LockInFullscreen")
  (Variables|/Script/Engine.PlayerController|SetbShowMouseCursor _returnvalue true))

(fn GetWidget
  (params (Name :type String))
  (bind _returnvalue (Class|WidgetManager|GetWidget (Variables|Default|GetwidgetManager) Name))
  (return _returnvalue))

(event EventInitWidgetManager
  (Utilities|MAddWidget "Loading" "/Game/ASSETS/MainMenu/LoadingScreen/FinalPoolLoadingScreenBP.FinalPoolLoadingScreenBP_C" 9000)
  (Class|SefaPoolGameInstance|ShowLoadingScreen)
  (Utilities|FlowControl|Delay 0.1)
  (Utilities|FlowControl|Sequence
    (:then_0
      (Utilities|FlowControl|Sequence
        (:then_0
          (Utilities|MAddWidget "MainShop" "/Game/ASSETS/UI/Shop/NewShop/Shop/MainShopWidgetBP_New.MainShopWidgetBP_New_C" 1)
          (Utilities|MAddWidget "MainMenu" "/Game/ASSETS/MainMenu/FinalMenuWidgetBP.FinalMenuWidgetBP_C")
          (Utilities|MAddWidget "PauseMenu" "/Game/ASSETS/PauseMenu/PauseMenuWB.PauseMenuWB_C" 10)
          (Utilities|MAddWidget "InGameShop" "/Game/ASSETS/UI/Shop/NewShop/Shop/FinalInGameShopWidgetBP.FinalInGameShopWidgetBP_C" 11)
          (Utilities|MAddWidget "RemoteMessages" "/Game/ASSETS/MainMenu/Messages/FinalMessagesMenuWidgetBP.FinalMessagesMenuWidgetBP_C" 12)
          (Utilities|MAddWidget "AppInfo" "/Game/ASSETS/MainMenu/OldStuff/NewAppVersionMenuWidgetBP.NewAppVersionMenuWidgetBP_C" 12)
          (Utilities|MAddWidget "ChampionshipLeaderboardMenu" "/Game/ASSETS/PlayMenu/FinalChampionshipLeaderboardWidgetBP.FinalChampionshipLeaderboardWidgetBP_C" 2)
          (Utilities|MAddWidget "Popup" "/Game/ASSETS/MainMenu/Popups/PopupWidgetBP.PopupWidgetBP_C" 13))
        (:then_1
          (Utilities|MAddWidget "UserMenu" "/Game/ASSETS/UI/UserMenu/FinalUserMenuWidgetBP.FinalUserMenuWidgetBP_C" 10)
          (Utilities|MAddWidget "BuyConfirmation")
          (Utilities|MAddWidget "ChooseTheMap" "/Game/ASSETS/ChooseTheMap/ChooseTheMap.ChooseTheMap_C")
          (Utilities|MAddWidget "SelectedContest" "/Game/ASSETS/ContestMenu/SelectedContestWidgetBP.SelectedContestWidgetBP_C" 3)
          (Utilities|MAddWidget "LoseScreen" "/Game/ASSETS/MainMenu/LoseScreenWidget.LoseScreenWidget_C" 9001)
          (Utilities|MAddWidget "Friends" "/Game/ASSETS/MainMenu/Friends/FriendMenuWidgetBP.FriendMenuWidgetBP_C" 12)
          (Utilities|MAddWidget "SpectatingMenu" "/Game/ASSETS/PlayMenu/SpectatingMenuWidgetBP.SpectatingMenuWidgetBP_C" 2)
          (Utilities|MAddWidget "PreLogin" "/Game/ASSETS/AuthenticationWidgets/PreLogin_WB.PreLogin_WB_C")
          (Utilities|MAddWidget "InteractivePopup" "/Game/ASSETS/MainMenu/Popups/InteractivePopupWidgetBP.InteractivePopupWidgetBP_C" 13))
        (:then_2
          (Utilities|MAddWidget "ContestMenu" "/Game/ASSETS/ContestMenu/ContestMenuWidgetBP.ContestMenuWidgetBP_C" 2)
          (Utilities|MAddWidget "PlayMenu" "/Game/ASSETS/PlayMenu/PlayMenuWidgetBP.PlayMenuWidgetBP_C" 1)
          (Utilities|MAddWidget "Settings" "/Game/ASSETS/UI/Settings/WBP_MainSettingsWidget.WBP_MainSettingsWidget_C" 11)
          (Utilities|MAddWidget "Registration" "/Game/ASSETS/AuthenticationWidgets/Registration_WB.Registration_WB_C" 1)
          (Utilities|MAddWidget "WinScreen" "/Game/ASSETS/MainMenu/WinScreenWidget.WinScreenWidget_C" 9001)
          (Utilities|MAddWidget "NewRemoteMessage" "/Game/ASSETS/MainMenu/Messages/FinalNewRemoteMessagePopup.FinalNewRemoteMessagePopup_C" 11)
          (Utilities|MAddWidget "ReplayMenu" "/Game/ASSETS/MainMenu/Replays/FinalReplaysMenuWidgetBP.FinalReplaysMenuWidgetBP_C" 12)
          (Utilities|MAddWidget "ContestLeaderboardMenu" "/Game/ASSETS/PlayMenu/FinalContestLeaderboardMenuWidgetBP.FinalContestLeaderboardMenuWidgetBP_C" 2)
          (Utilities|MAddWidget "Purchases" "/Game/ASSETS/MainMenu/Purchase/PurchaseMenuWidgetBP.PurchaseMenuWidgetBP_C" 12))
        (:then_3
          (Utilities|MAddWidget "Login" "/Game/ASSETS/AuthenticationWidgets/Login_WB.Login_WB_C")
          (Utilities|MAddWidget "ChooseStake" "/Game/ASSETS/PreGameWidgets/ChooseStake.ChooseStake_C")
          (Utilities|MAddWidget "ChooseDifficulty" "/Game/ASSETS/ChooseDifficulty/ChooseDifficulty.ChooseDifficulty_C" 4)
          (Utilities|MAddWidget "SensitivityMenu" "/Game/ASSETS/SensitivityMenu/SensitivityMenuWB.SensitivityMenuWB_C")
          (Utilities|MAddWidget "MainUserMenu" "/Game/ASSETS/MainMenu/OldStuff/NewUserMenuWidgetBP.NewUserMenuWidgetBP_C")
          (Utilities|MAddWidget "ProfileMenu" "/Game/ASSETS/MainMenu/OldStuff/NewProfileMenuWidgetBP.NewProfileMenuWidgetBP_C" 12)
          (Utilities|MAddWidget "InviteMenu" "/Game/ASSETS/PlayMenu/InviteMenuWidgetBp.InviteMenuWidgetBP_C" 2)
          (Utilities|MAddWidget "EquipmentMenu" "/Game/ASSETS/MainMenu/Equipment/EquipmentMenuWidgetBP.EquipmentMenuWidgetBP_C" 12))))
    (:then_1
      (Utilities|FlowControl|Sequence
        (:then_0
          (Variables|Default|SetCaching true)
          (Class|WidgetManager|InitandStartCaching (Variables|Default|GetwidgetManager) self)
          (Variables|Default|SetPostCachingLoadingScreenRemovalRequest false))
        (:then_1
          (Utilities|FlowControl|Delay 2.0)
          (Class|WidgetManager|EndCaching (Variables|Default|GetwidgetManager))
          (Variables|Default|SetCaching false)
          (if (Variables|Default|GetPostCachingLoadingScreenRemovalRequest)
            (Variables|Default|SetPostCachingLoadingScreenRemovalRequest false))
          (Class|SefaPoolGameInstance|HideLoadingScreen)
          (if (Variables|Default|GetPostCachingShowWidget)
            (CallFunction|ShowWidget (Variables|Default|GetPostCachingWidgetName))))))))
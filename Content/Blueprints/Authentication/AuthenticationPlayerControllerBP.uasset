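; Player controller for the authentication stage, handling login, registration and offline play on the way to the main menu, in portrait orientation.
; On player entry, a command-line user_id triggers automatic login with a fixed password; otherwise it checks the server connection.
; Successful login or connection requests main-menu data, saves it and opens the menu in online mode.
; Callback events drive GameInstance widgets and popups; connection failure or offline play still opens the menu.
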(event Custom|SuccesfulConnection
  ;[1 1 1] Processing entered player
  (CallFunction|ProcessRequestEntryDatafromMainMenu))

(event Custom|EntryRequestSuccseful
  (bind _gameinstance (Variables|Default|GetGameInstance))
  ;[1 1 1] Processing getting initial data for main menu
  (Class|SefaPoolData|FullSave (Variables|/Script/SefaPool.SefaPoolGameInstance|Getdata (Variables|Default|GetGameInstance)))
  (Class|SefaPoolGameInstance|ShowLoadingScreen _gameinstance)
  (bind _widget (Default|GetWidget _gameinstance "MainMenu"))
  (bind _asnew_menu_widget_bp (Utilities|Casting|CastToNewMenuWidgetBP _widget)
    (:then
      (Default|SetOnlineMode _asnew_menu_widget_bp))
    (:CastFailed
      _))
  (Default|ShowWidget _gameinstance "MainMenu")
  (Default|HideWidget _gameinstance "Login")
  (Default|HideWidget _gameinstance "PreLogin")
  (Default|HideWidget _gameinstance "Registration"))

(event Custom|RegistrationUnsuccesful
  ;[1 1 1] Processing registration
  (Class|SefaPoolGameInstance|ShowPopup (Variables|Default|GetGameInstance) "Registration" "This username is already taken 
Please select another one" "OK"))

(event Custom|OfflinePlay
  ;[1 1 1] Processing entered player
  (Class|AuthenticationPlayerController|Offline)
  (Default|HideWidget (Variables|Default|GetGameInstance) "PreLogin")
  (Default|ShowWidget (Variables|Default|GetGameInstance) "MainMenu"))

(event Custom|EntryRequestUnsuccesful
  (bind _gameinstance (Variables|Default|GetGameInstance))
  ;[1 1 1] Processing getting initial data for main menu
  (Class|SefaPoolGameInstance|HideLoadingScreen _gameinstance)
  (Default|ShowWidget _gameinstance "PreLogin"))

(event Custom|LoginUnsuccesful
  (bind _gameinstance (Variables|Default|GetGameInstance))
  ;[1 1 1] Processing login request
  (Class|SefaPoolGameInstance|HideLoadingScreen _gameinstance)
  (Default|ShowWidget _gameinstance "Login")
  (Class|SefaPoolGameInstance|ShowPopup (Variables|Default|GetGameInstance) "Login" "Failed to login 
This login-password pair does not exist" "Ok"))

(event Custom|LoginSuccesful
  ;[1 1 1] Processing login request
  (CallFunction|ProcessRequestEntryDatafromMainMenu))

(event Custom|ProcessRequestEntryDataFromMainMenu
  ;[1 1 1] Processing getting initial data for main menu
  (Class|AuthenticationPlayerController|RequestEntryDataforMainMenu (delegate Custom|EntryRequestSuccseful) (delegate Custom|EntryRequestUnsuccesful)))

(event Custom|UnsuccesfulConnection
  ;[1 1 1] Processing entered player
  (Class|SefaPoolGameInstance|ShowPopup (Variables|Default|GetGameInstance) "Connectivity" "Could not connect to the server 
Please check your internet connection" "OK")
  (Default|HideWidget (Variables|Default|GetGameInstance) "PreLogin")
  (Default|ShowWidget (Variables|Default|GetGameInstance) "MainMenu"))

(event Custom|RegistrationSuccesful
  ;[1 1 1] Processing registration
  (Class|SefaPoolGameInstance|ShowPopup (Variables|Default|GetGameInstance) "Registration" "Your registration was successful 
You can now login with your credentials" "OK")
  (Default|SwapWidgets (Variables|Default|GetGameInstance) "Login" "Registration"))

(event EventProcessEnteredPlayer
  (bind _returnvalue (Utilities|GetCommandLine))
  (bind _outparams (Class|KismetSystemLibrary|ParseCommandLine _returnvalue))
  (if (.ReturnValue (Utilities|Map|Find _outparams "user_id"))
    (Class|AuthenticationPlayerController|RequestLogin (.Value (Utilities|Map|Find _outparams "user_id")) "1" (delegate Custom|LoginSuccesful) (delegate Custom|LoginUnsuccesful))
    (else
      ;[1 1 1] Processing entered player
      (bind _asmain_game_instance (Utilities|Casting|CastToMainGameInstance (Game|GetGameInstance)))
      (Variables|Default|SetGameInstance _asmain_game_instance)
      (bind _asauthentication_player_controller (Utilities|Casting|CastToAuthenticationPlayerController (Game|GetPlayerController 0)))
      (Variables|Default|SetPlayerController _asauthentication_player_controller)
      (Class|AuthenticationPlayerController|RequestCheckConnectionwithServer (Variables|Default|GetPlayerController) (delegate Custom|SuccesfulConnection) (delegate Custom|UnsuccesfulConnection)))))

(event EventProcessLogin
  (params (username :type String) (password :type String))
  (bind _gameinstance (Variables|Default|GetGameInstance))
  ;[1 1 1] Processing login request
  (Class|SefaPoolGameInstance|ShowLoadingScreen _gameinstance)
  (Default|HideWidget _gameinstance "Login")
  (Class|AuthenticationPlayerController|RequestLogin (Variables|Default|GetPlayerController) username password (delegate Custom|LoginSuccesful) (delegate Custom|LoginUnsuccesful)))

(event EventProcessRegistration
  (params (data :type Registration%20Data%20Structure%20%28by%20ref%29))
  ;[1 1 1] Processing registration
  (Class|AuthenticationPlayerController|RequestRegistration data (delegate Custom|RegistrationSuccesful) (delegate Custom|RegistrationUnsuccesful)))

(event EventBeginPlay
  (bind _assefa_pool_game_instance (Utilities|Casting|CastToSefaPoolGameInstance (Game|GetGameInstance)))
  (Class|SefaPoolGameInstance|SwitchtoOrientation _assefa_pool_game_instance "ORIENTATION_PORTRAIT"))

(fn ConstructionScript)
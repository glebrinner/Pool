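; BP_PoolMPPlayer is the pool player Blueprint, handling timeline-driven camera transitions between the cue-ball view and a walk-around view.
; Border reset eases the camera toward the view spline near its far end or the default position near its start.
; Walk mode blends onto a separate spline looking at a fixed point; leaving it blends back to face the cue ball.
; Tick prints the walk-view spline position for debugging.
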(event EventTick
  (params (DeltaSeconds :type Float%20%28single-precision%29))
  (Development|PrintString (Utilities|String|ToString(Float) (Variables|Default|GetWalkCameraViewStack)) true false "(R=0.000000,G=0.143530,B=1.000000,A=1.000000)" DeltaSeconds))

(event EventBPResetCamerafromBorder
  (if (> (Variables|Default|GetCameraViewStack) 0.9)
    (bind _value (Timeline|Timeline_0 PlayFromStart)
      (:Update
        (Transformation|SetRelativeLocation (Variables|Default|Getcamera) (Math|Vector|Lerp(Vector) (Variables|/Script/Engine.SceneComponent|GetRelativeLocation (Variables|Default|Getcamera)) (Spline|GetLocationatTime (Variables|Default|GetCameraViewSpline) 0.9 "World" false) _value) false false)))
    (elif (< (Variables|Default|GetCameraViewStack) 0.1)
      (bind _value_2 (Timeline|Timeline_1 PlayFromStart)
        (:Update
          (Transformation|SetRelativeLocation (Variables|Default|Getcamera) (Math|Vector|Lerp(Vector) (Variables|/Script/Engine.SceneComponent|GetRelativeLocation (Variables|Default|Getcamera)) (Variables|Default|GetDefaultCameraPos) _value_2) false false))))))

(event EventBPBlendCameratoWalkMode
  (params (IsActive :type Boolean))
  (bind _camera (Variables|Default|Getcamera))
  (bind _camera_2 (Variables|Default|Getcamera))
  (if IsActive
    (bind _value (Timeline|Timeline_2 PlayFromStart)
      (:Update
        (Transformation|SetWorldLocation _camera (Math|Vector|Lerp(Vector) (Transformation|GetWorldLocation _camera) (Spline|GetLocationatTime (Variables|Default|GetWalkCameraViewSpline) (Variables|Default|GetWalkCameraViewStack) "World" false) _value) false false)
        (Transformation|SetWorldRotation _camera (Math|Rotator|FindLookatRotation (Transformation|GetWorldLocation _camera) (Math|Vector|MakeVector 0.0 0.0 75.0)) false false)))
    (else
      (bind _value_2 (Timeline|Timeline_3 PlayFromStart)
        (:Update
          (Transformation|SetRelativeLocation _camera_2 (Math|Vector|Lerp(Vector) (Variables|/Script/Engine.SceneComponent|GetRelativeLocation _camera_2) (Spline|GetLocationatTime (Variables|Default|GetCameraViewSpline) (Variables|Default|GetCameraViewStack) "World" false) _value_2) false false)
          (Transformation|SetWorldRotation _camera_2 (Math|Rotator|Lerp(Rotator) (Transformation|GetWorldRotation _camera_2) (Math|Rotator|FindLookatRotation (Transformation|GetWorldLocation _camera_2) (Transformation|GetActorLocation (Variables|Default|GetcueBall))) _value_2 true) false false))))))

(fn ConstructionScript)